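; A two-way room Blueprint, apparently the left-right variant, that registers the navigation nodes placed inside it.
; On BeginPlay it gathers all child actors, including descendants, and filters them to NavigationNode.
; It casts itself to Room, sets that as each node's owning room and adds the node to ListOfNavNodes, printing a message if a cast fails.
; Overlap, Tick and the construction script are empty.
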(event `self.ReceiveBeginPlay`
  (bind _filteredarray (`KismetArrayLibrary.FilterArray` (`self.GetAllChildActors` true) "/Script/AdvGamesProgramming.NavigationNode"))
  (for _array_element _filteredarray
    (bind _asnavigation_node (cast `NavigationNode` _array_element)
      (:`then`
        (bind _asroom (cast `Room` self)
          (:`then`
            (set `NavigationNode.Room` _asroom _asnavigation_node)
            (`KismetArrayLibrary.Array_Add` (`self.ListOfNavNodes`) _asnavigation_node))
          (:`CastFailed`
            (`KismetSystemLibrary.PrintString` "Cast to room failed"))))
      (:`CastFailed`
        (`KismetSystemLibrary.PrintString` "Cast to navnode failed")))))

(fn `UserConstructionScript`)