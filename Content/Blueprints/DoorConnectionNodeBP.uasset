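; Door connection node actor that finds a neighboring door node through an on-demand proximity check.
; CheckForNearbyDoorNode runs a sphere overlap around the node, filtered to world-dynamic DoorConnectionNode actors and ignoring its owner, and returns the first hit after a cast.
; The check draws a debug sphere and prints success or failure messages; the event graph and construction script are empty.
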(fn `CheckForNearbyDoorNode`
  (returns (ReturnValue :type "DoorConnectionNode Object Reference"))
  (bind _returnvalue (`self.K2_GetActorLocation`))
  (`KismetSystemLibrary.DrawDebugSphere` _returnvalue 225.0 12 (struct :`R` 1.0 :`G` 1.0 :`B` 1.0 :`A` 1.0) 20.0)
  (bind (_outactors _returnvalue_2) (`KismetSystemLibrary.SphereOverlapActors` _returnvalue 225.0 (`|MakeArray` "ObjectTypeQuery2" :!type "EObjectTypeQuery Enum") "/Script/AdvGamesProgramming.DoorConnectionNode" (`|MakeArray` (`self.GetOwner`))))
  (if _returnvalue_2
    (bind _asdoor_connection_node (cast `DoorConnectionNode` (`|GetArrayItem` _outactors))
      (:`then`
        (`KismetSystemLibrary.PrintString` "Door Touched")
        (return _asdoor_connection_node))
      (:`CastFailed`
        (`KismetSystemLibrary.PrintString` "Cast failed" true true (struct :`G` 0.66 :`B` 1.0 :`A` 1.0) 10.0)))
    (else
      (`KismetSystemLibrary.PrintString` "Touch failed" true true (struct :`G` 0.66 :`B` 1.0 :`A` 1.0) 10.0))))

(fn `UserConstructionScript`)