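; Procedural level generation Blueprint that checks the room at its location and swaps it for one with a bottom when needed.
; CheckRoom runs a small sphere overlap for Room actors and tests the first hit's RoomType.
; Rooms outside the two accepted types are destroyed through RoomDestruction, then SpawnRoomWithBottom spawns the replacement.
; A debug sphere and printed messages show each check's result.
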(event `self.CheckRoom`
  (bind _returnvalue (`self.K2_GetActorLocation`))
  (`KismetSystemLibrary.DrawDebugSphere` _returnvalue 50.0 12 (struct :`R` 1.0 :`G` 1.0 :`B` 1.0 :`A` 1.0) 3.0)
  (bind (_outactors _returnvalue_2) (`KismetSystemLibrary.SphereOverlapActors` _returnvalue 50.0 (`|MakeArray` "ObjectTypeQuery2" :!type "EObjectTypeQuery Enum") "/Script/AdvGamesProgramming.Room"))
  (if _returnvalue_2
    (bind _asroom (cast `Room` (`|GetArrayItem` _outactors)))
    (bind _roomtype (`Room.RoomType` _asroom))
    (if (and (!= _roomtype 1) (!= _roomtype 3))
      (`Room.RoomDestruction` _asroom)
      (`KismetSystemLibrary.PrintString` "Room Destroyed")
      (`self.SpawnRoomWithBottom`)
      (else
        (`KismetSystemLibrary.PrintString` "No Room destroyed")))
    (else
      (`KismetSystemLibrary.PrintString` "Diidn't touch room"))))

(fn `UserConstructionScript`)