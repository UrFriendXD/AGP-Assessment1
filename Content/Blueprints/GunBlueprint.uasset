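; Gun actor Blueprint that fires predicted-projectile shots for its parent player character.
; Fire traces a projectile path from the muzzle instead of spawning a projectile, draws it for debugging, plays a sound and the character's arms fire montage.
; An actor hit with a HealthComponent takes bullet damage, with debug prints of the result.
; Tick counts down the fire-rate cooldown that re-enables firing.
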(event `self.ReceiveTick`
  (params (DeltaSeconds :type "Float (single-precision)"))
  (if (not (`self.bCanFire`))
    (bind _output_get (set `self.TimeTillNextShot` (- (`self.TimeTillNextShot`) DeltaSeconds)))
    (if (<= _output_get 0.0)
      (set `self.bCanFire` true))))

(fn `Fire`
  (params (LaunchDirection :type "Vector Structure"))
  (bind _returnvalue (`SceneComponent.K2_GetComponentLocation` (`self.MuzzlePosition`)))
  (if (`self.bCanFire`)
    (set `self.bCanFire` false)
    (set `self.TimeTillNextShot` (`self.FireRate`))
    (bind _outhit (`GameplayStatics.Blueprint_PredictProjectilePath_ByTraceChannel` :`StartPos` _returnvalue :`LaunchVelocity` (* LaunchDirection (`self.MuzzleVelocity`)) :`ProjectileRadius` 1.0 :`DrawDebugType` "ForDuration" :`DrawDebugTime` 4.0))
    (`GameplayStatics.PlaySoundAtLocation` "/Game/Assets/Audio/FirstPersonTemplateWeaponFire02.FirstPersonTemplateWeaponFire02" _returnvalue (struct) 1.0 1.0 0.0 null null null)
    (bind _asplayer_character_blueprint (cast `/Game/Blueprints/PlayerCharacterBlueprint` (`self.GetParentActor`)))
    (`AnimInstance.Montage_Play` (`SkeletalMeshComponent.GetAnimInstance` (`/Game/Blueprints/PlayerCharacterBlueprint.Arms` _asplayer_character_blueprint)) "/Game/Assets/Arms/Animations/FirstPersonFire_Montage.FirstPersonFire_Montage" 1.0 "MontageLength" 0.0 true)
    (bind (_bblockinghit _binitialoverlap _time _distance _location _impactpoint _normal _impactnormal _physmat _hitactor) (`GameplayStatics.BreakHitResult` _outhit))
    (if (`KismetSystemLibrary.IsValid` _hitactor)
      (bind _returnvalue_2 (`self.GetComponentByClass` _hitactor "/Script/AdvGamesProgramming.HealthComponent"))
      (if (`KismetSystemLibrary.IsValid` _returnvalue_2)
        (`HealthComponent.OnTakeDamage` _returnvalue_2 (`self.BulletDamage`))
        (`KismetSystemLibrary.PrintString` (`KismetStringLibrary.Conv_DoubleToString` (`HealthComponent.CurrentHealth` _returnvalue_2)) true false)
        (else
          (`KismetSystemLibrary.PrintString` "Did not hit actor with health component" true false))))))

(fn `UserConstructionScript`)