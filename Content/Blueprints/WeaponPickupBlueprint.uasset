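; Weapon pickup actor that passes its stats and rarity look to the gun of the player or enemy character that picks it up.
; On BeginPlay it calls OnGenerate on authority only, then colors its skeletal mesh by Rarity.
; OnPickup copies the stats and material onto the character's child-actor gun, then destroys the pickup.
; Enemies receive scaled-down stats and have their rounds remaining set; players get full stats.
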(event `self.ReceiveBeginPlay`
  (bind _skeletalmesh (`self.SkeletalMesh`))
  (`/Engine/EditorBlueprintResources/ActorMacros.Switch Has Authority`
    (:`Authority`
      (`self.OnGenerate`))
    (:`Remote`
      _))
  (switch `WeaponPickupRarity` (`self.Rarity`)
    (:`LEGENDARY`
      (`PrimitiveComponent.SetMaterial` _skeletalmesh 0 "/Game/Materials/Gold.Gold"))
    (:`MASTER`
      (`PrimitiveComponent.SetMaterial` _skeletalmesh 0 "/Game/Materials/Purple.Purple"))
    (:`RARE`
      (`PrimitiveComponent.SetMaterial` _skeletalmesh 0 "/Game/Materials/Blue.Blue"))
    (:`COMMON`
      (`PrimitiveComponent.SetMaterial` _skeletalmesh 0 "/Game/Materials/White.White"))))

(event `self.OnPickup`
  (params (ActorThatPickedUp :type "Actor Object Reference"))
  (bind _returnvalue (/ (`self.MagazineSize`) 2))
  (bind _asplayer_character_blueprint (cast `/Game/Blueprints/PlayerCharacterBlueprint` ActorThatPickedUp)
    (:`then`
      (bind _asgun_blueprint (cast `/Game/Blueprints/GunBlueprint` (`ChildActorComponent.ChildActor` (`/Game/Blueprints/PlayerCharacterBlueprint.Gun` _asplayer_character_blueprint))))
      (set `/Game/Blueprints/GunBlueprint.BulletDamage` (`self.BulletDamage`) _asgun_blueprint)
      (set `/Game/Blueprints/GunBlueprint.MuzzleVelocity` (`self.MuzzleVelocity`) _asgun_blueprint)
      (set `/Game/Blueprints/GunBlueprint.MagazineSize` (`self.MagazineSize`) _asgun_blueprint)
      (set `/Game/Blueprints/GunBlueprint.WeaponAccuracy` (`self.WeaponAccuracy`) _asgun_blueprint)
      (`PrimitiveComponent.SetMaterial` (`/Game/Blueprints/GunBlueprint.GunMesh` _asgun_blueprint) 0 (`PrimitiveComponent.GetMaterial` (`self.SkeletalMesh`) 0))
      (`self.K2_DestroyActor`))
    (:`CastFailed`
      (bind _asenemy_character_blueprint (cast `/Game/Blueprints/EnemyCharacterBlueprint` ActorThatPickedUp))
      (bind _asgun_blueprint_2 (cast `/Game/Blueprints/GunBlueprint` (`ChildActorComponent.ChildActor` (`/Game/Blueprints/EnemyCharacterBlueprint.Gun` _asenemy_character_blueprint))))
      (set `/Game/Blueprints/GunBlueprint.BulletDamage` (/ (`self.BulletDamage`) 3.0) _asgun_blueprint_2)
      (set `/Game/Blueprints/GunBlueprint.MuzzleVelocity` (/ (`self.MuzzleVelocity`) 3.0) _asgun_blueprint_2)
      (set `/Game/Blueprints/GunBlueprint.MagazineSize` _returnvalue _asgun_blueprint_2)
      (set `/Game/Blueprints/GunBlueprint.WeaponAccuracy` (/ (`self.WeaponAccuracy`) 3.0) _asgun_blueprint_2)
      (set `/Game/Blueprints/GunBlueprint.RoundsRemainingInMagazine` _returnvalue _asgun_blueprint_2)
      (`PrimitiveComponent.SetMaterial` (`/Game/Blueprints/GunBlueprint.GunMesh` _asgun_blueprint_2) 0 (`PrimitiveComponent.GetMaterial` (`self.SkeletalMesh`) 0))
      (`self.K2_DestroyActor`))))

(fn `UserConstructionScript`)